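; BP_BossSandFloor is an actor, named as the sand floor of a boss encounter.
; On BeginPlay it casts the game mode to BP_GameMode and stores itself in that mode's SandFloor variable so other logic can reach it.
; It has no other active logic, as the overlap and tick events are disabled and the construction script only calls its parent.
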(event EventBeginPlay
  (|CallParentFunction)
  (bind _asbp_game_mode (Utilities|Casting|CastToBP_GameMode (Game|GetGameMode)))
  (Variables|/Game/BP_GameMode.BP_GameMode_C|SetSandFloor _asbp_game_mode self))

(event Collision|EventActorBeginOverlap
  (params (OtherActor :type Actor%20Object%20Reference))
  (|CallParentFunction OtherActor) ; This node is disabled and will not be called.\nDrag off pins to build functionality.
)

(event EventTick
  (params (DeltaSeconds :type Float%20%28single-precision%29))
  (|CallParentFunction DeltaSeconds) ; This node is disabled and will not be called.\nDrag off pins to build functionality.
)

(fn ConstructionScript
  (|CallParentFunction))