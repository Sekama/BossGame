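; Actor component that flashes a colored, emissive damage overlay on its owner when ApplyEffect is called.
; On BeginPlay it puts a dynamic M_DamageOverlay material on the owner's mesh, adding a chamfer cube mesh if none exists.
; ApplyEffect restarts a timer that serves as a clock, and Tick uses its elapsed time to drive opacity along a half-sine fade in and out.
; Tick also reapplies color and emission every frame.
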(event Custom|ApplyEffect
  (if (Utilities|Time|IsValidTimerHandle (Variables|Default|GetEffectTimer))
    (Utilities|Time|ClearandInvalidateTimerbyHandle (Variables|Default|GetEffectTimer)))
  (bind _returnvalue (Utilities|Time|SetTimerbyFunctionName 0 "Managing Effect" (Variables|DefaultParam|GetDuration)))
  (Variables|Default|SetEffectTimer _returnvalue))

(event EventBeginPlay
  (bind _returnvalue (Components|GetOwner))
  (bind _returnvalue_2 (Actor|GetComponentbyClass _returnvalue "/Script/Engine.MeshComponent"))
  (Utilities|IsValid _returnvalue_2
    (:Is%20Valid
      (Variables|Default|SetOwnerMesh _returnvalue_2)
      (bind _returnvalue_3 (Rendering|Material|CreateDynamicMaterialInstance "/Game/Materials/Characters/M_DamageOverlay.M_DamageOverlay" "None" "None" :!class /Script/Engine.KismetMaterialLibrary :!label _label))
      (bind _output_get (Variables|Components|SetM_Overlay _returnvalue_3))
      (Rendering|Material|SetOverlayMaterial (Variables|Default|GetOwnerMesh) _output_get :!class /Script/Engine.MeshComponent)
      (CallFunction|SetAllParameterValues)
      (CallFunction|SetOpacity 0.0))
    (:Is%20Not%20Valid
      (bind _returnvalue_4 (Game|AddComponentbyClass _returnvalue "/Script/Engine.StaticMeshComponent" false))
      (bind _output_get_2 (Variables|Default|SetOwnerMesh _returnvalue_4))
      (bind _asstatic_mesh_component (Utilities|Casting|CastToStaticMeshComponent _output_get_2)
        (:then
          (Components|StaticMesh|SetStaticMesh _asstatic_mesh_component "/Game/LevelPrototyping/Meshes/SM_ChamferCube.SM_ChamferCube")
          (goto _label))
        (:CastFailed
          (Development|PrintString (Utilities|String|Append "Cannot add a mesh to the actor - " (Utilities|GetObjectName _returnvalue))))))))

(event EventTick
  (params (DeltaSeconds :type Float%20%28single-precision%29))
  (CallFunction|SetAllParameterValues)
  (if (Utilities|Time|IsValidTimerHandle (Variables|Default|GetEffectTimer))
    (CallFunction|ManagingEffect)))

(fn ManagingEffect
  (bind _effecttimer (Variables|Default|GetEffectTimer))
  (if (not (Utilities|Time|IsTimerActivebyHandle _effecttimer))
    (CallFunction|SetOpacity 0.0 :!label _label)
    (Utilities|Time|ClearandInvalidateTimerbyHandle (Variables|Default|GetEffectTimer))
    (else
      (CallFunction|SetOpacity (* (Math|Trig|Sin(Radians) (* (/ (Class|KismetSystemLibrary|GetTimerElapsedTimeHandle _effecttimer) (Variables|DefaultParam|GetDuration)) (Math|Trig|GetPI))) (Variables|DefaultParam|GetOpacity)))
      (if (<= (Utilities|Time|GetTimerRemainingTimebyHandle (Variables|Default|GetEffectTimer)) 0.0)
        (goto _label)))))

(fn SetEmission
  (params (Emission :type Float%20%28double-precision%29))
  (Rendering|Material|SetScalarParameterValue (Variables|Components|GetM_Overlay) "EmissiveStrength" Emission :!class /Script/Engine.MaterialInstanceDynamic))

(fn SetOpacity
  (params (Opacity :type Float%20%28double-precision%29))
  (Rendering|Material|SetScalarParameterValue (Variables|Components|GetM_Overlay) "Opacity" Opacity :!class /Script/Engine.MaterialInstanceDynamic))

(fn SetColor
  (params (Color :type Linear%20Color%20Structure))
  (Rendering|Material|SetVectorParameterValue (Variables|Components|GetM_Overlay) "Color" Color :!class /Script/Engine.MaterialInstanceDynamic))

(fn SetAllParameterValues
  (CallFunction|SetEmission (Variables|MaterialParam|GetEmission))
  (CallFunction|SetColor (Variables|MaterialParam|GetColor)))