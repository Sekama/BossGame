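; Actor component that flashes a damage overlay on its owner's meshes when ApplyEffect is called.
; On BeginPlay it creates a dynamic M_DamageOverlay instance and, absent assigned meshes, gathers the owner's mesh components or adds a chamfer cube.
; It drops entries lacking static or skeletal mesh assets before applying the overlay.
; A restartable timer drives Tick, which refreshes color and emission and pulses opacity along a half-sine over Duration.
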(event Custom|ApplyEffect
  (Handling|ReevaluteMeshItems)
  (Overlay|ReapplyMaterialOverlay)
  (if (Utilities|Time|IsValidTimerHandle (Variables|Default|GetEffectTimer)) ; Reset timer if it already exists
    (Utilities|Time|ClearandInvalidateTimerbyHandle (Variables|Default|GetEffectTimer)))
  (bind _returnvalue (Utilities|Time|SetTimerbyFunctionName 0 "HandleMaterialEffect" (Variables|MaterialParams|GetDuration)))
  (Variables|Default|SetEffectTimer _returnvalue))

(event Custom|GetAllMeshItems
  (bind _returnvalue (Components|GetOwner))
  (bind _returnvalue_2 (Actor|GetComponentsByClass _returnvalue "/Script/Engine.MeshComponent"))
  (if (Utilities|Array|IsNotEmpty _returnvalue_2)
    (CallFunction|SetMeshItems _returnvalue_2)
    (else
      (bind _meshitems (Mesh|CreateDefaultMesh))
      (CallFunction|SetMeshItems _meshitems))))

(event Custom|SetMeshItems
  (params (MeshComps :type Array%20of%20Mesh%20Component%20Object%20References))
  (for _array_element (Variables|Default|GetMeshObjects)
    (Handling|ClearOverlayMaterial _array_element))
  (Utilities|Array|Clear (Variables|Default|GetMeshObjects))
  (Variables|Default|SetMeshObjects MeshComps)
  (Handling|ReevaluteMeshItems)
  (Overlay|ReapplyMaterialOverlay))

(event Custom|UpdateMeshItems
  (params (MeshComps :type Array%20of%20Mesh%20Component%20Object%20References))
  (for _array_element MeshComps
    (Utilities|Array|AddUnique (Variables|Default|GetMeshObjects) _array_element))
  (Overlay|ReapplyMaterialOverlay))

(event Custom|RemoveMeshItem
  (params (MeshComp :type Mesh%20Component%20Object%20Reference))
  (Handling|ClearOverlayMaterial MeshComp)
  (bind _returnvalue (Utilities|Array|RemoveItem (Variables|Default|GetMeshObjects) MeshComp))
  (if _returnvalue
    (Development|PrintString "Successfully removed an item")))

(event EventBeginPlay
  (if (not (Variables|Components|GetHasInit?))
    (Utilities|Array|Clear (Variables|Default|GetMeshObjects))
    (Variables|Components|SetHasInit? true)
    (if (not (Utilities|IsValid (Variables|Components|GetDyanmicOverlay_M)))
      (bind _returnvalue (Rendering|Material|CreateDynamicMaterialInstance "/Game/Materials/Characters/M_DamageOverlay.M_DamageOverlay" "None" "None" :!class /Script/Engine.KismetMaterialLibrary))
      (Variables|Components|SetDyanmicOverlay_M _returnvalue)
      (Material|ApplyMaterialDefaults)
      (Material|SetMaterialOpacity 0.0)
      (Utilities|FlowControl|DelayUntilNextTick)
      (if (Utilities|Array|IsNotEmpty (Variables|Default|GetMeshObjects))
        (Overlay|ReapplyMaterialOverlay)
        (else
          (CallFunction|GetAllMeshItems))))))

(event EventTick
  (params (DeltaSeconds :type Float%20%28single-precision%29))
  (Material|ApplyMaterialDefaults)
  (if (Utilities|Time|IsValidTimerHandle (Variables|Default|GetEffectTimer))
    (Handling|HandleMaterialEffect)))

(fn HandleMaterialEffect
  (bind _effecttimer (Variables|Default|GetEffectTimer))
  (if (Utilities|IsValid (Variables|Components|GetDyanmicOverlay_M))
    (if (not (Utilities|Time|IsTimerActivebyHandle _effecttimer))
      (Material|SetMaterialOpacity 0.0 :!label _label)
      (Utilities|Time|ClearandInvalidateTimerbyHandle (Variables|Default|GetEffectTimer))
      (else
        (Material|SetMaterialOpacity (* (Math|Trig|Sin(Radians) (* (/ (Class|KismetSystemLibrary|GetTimerElapsedTimeHandle _effecttimer) (Variables|MaterialParams|GetDuration)) (Math|Trig|GetPI))) (Variables|MaterialParams|GetOpacity)))
        (if (<= (Utilities|Time|GetTimerRemainingTimebyHandle (Variables|Default|GetEffectTimer)) 0.0)
          (goto _label))))))

(fn SetMaterialEmission
  (params (Emission :type Float%20%28double-precision%29))
  (Rendering|Material|SetScalarParameterValue (Variables|Components|GetDyanmicOverlay_M) "EmissiveStrength" Emission :!class /Script/Engine.MaterialInstanceDynamic))

(fn SetMaterialOpacity
  (params (Opacity :type Float%20%28double-precision%29))
  (Rendering|Material|SetScalarParameterValue (Variables|Components|GetDyanmicOverlay_M) "Opacity" Opacity :!class /Script/Engine.MaterialInstanceDynamic))

(fn SetMaterialColor
  (params (Color :type Linear%20Color%20Structure))
  (Rendering|Material|SetVectorParameterValue (Variables|Components|GetDyanmicOverlay_M) "Color" Color :!class /Script/Engine.MaterialInstanceDynamic))

(fn ApplyMaterialDefaults
  (Material|SetMaterialEmission (Variables|MaterialParams|GetEmission))
  (Material|SetMaterialColor (Variables|MaterialParams|GetColor)))

(fn CreateDefaultMesh
  (bind _returnvalue (Game|AddComponentbyClass (Components|GetOwner) "/Script/Engine.StaticMeshComponent" false))
  (bind _output_get (Variables|Default|SetMeshObjects (Utilities|Array|MakeArray _returnvalue)))
  (Components|StaticMesh|SetStaticMesh _returnvalue "/Game/LevelPrototyping/Meshes/SM_ChamferCube.SM_ChamferCube")
  (return _output_get))

(fn ApplyMaterialOverlay
  (params (MeshComp :type Mesh%20Component%20Object%20Reference))
  (Rendering|Material|SetOverlayMaterial MeshComp (Variables|Components|GetDyanmicOverlay_M) :!class /Script/Engine.MeshComponent))

(fn ReapplyMaterialOverlay
  (Handling|ReevaluteMeshItems)
  (for _array_element (Variables|Default|GetMeshObjects)
    (Rendering|Material|SetOverlayMaterial _array_element (Variables|Components|GetDyanmicOverlay_M) :!class /Script/Engine.MeshComponent)))

(fn ClearOverlayMaterial
  (params (MeshItem :type Mesh%20Component%20Object%20Reference))
  (Utilities|IsValid MeshItem
    (:Is%20Valid
      (Rendering|Material|SetOverlayMaterial MeshItem 0 :!class /Script/Engine.MeshComponent))))

(fn ReevaluteMeshItems
  (Utilities|Array|Clear (LocalVariables|GetMeshItemsToRemove))
  (for _array_element (Variables|Default|GetMeshObjects)
    (bind _asskeletal_mesh_component (Utilities|Casting|CastToSkeletalMeshComponent _array_element)
      (:then
        (if (not (Utilities|IsValid (Components|SkeletalMesh|GetSkeletalMeshAsset _asskeletal_mesh_component)))
          (Utilities|Array|Add (LocalVariables|GetMeshItemsToRemove) 0 :!label _label)))
      (:CastFailed
        (bind _asstatic_mesh_component (Utilities|Casting|CastToStaticMeshComponent _array_element)
          (:then
            (if (not (Utilities|IsValid (Variables|/Script/Engine.StaticMeshComponent|GetStaticMesh _asstatic_mesh_component)))
              (goto _label)))
          (:CastFailed
            (goto _label))))))
  (if (not (Utilities|Array|IsEmpty (LocalVariables|GetMeshItemsToRemove)))
    (for _array_element_2 (LocalVariables|GetMeshItemsToRemove)
      (Utilities|Array|RemoveItem (Variables|Default|GetMeshObjects) _array_element_2))))