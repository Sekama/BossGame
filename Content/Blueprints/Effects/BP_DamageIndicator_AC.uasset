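; Actor component that flashes a pulsing damage overlay material on the owner's skeletal mesh when ApplyEffect is called.
; BeginPlay creates a dynamic M_DamageOverlay instance with configurable color and emission, initially transparent.
; ApplyEffect sets it as the mesh overlay, finding the owner's mesh if unset, and restarts a timer.
; Tick drives opacity from timer progress through an absolute sine over the set cycles, zeroing it when the timer ends.
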(event Custom|ApplyEffect
  (bind _returnvalue (Components|GetOwner))
  (bind _returnvalue_2 (Actor|GetComponentbyClass _returnvalue "/Script/Engine.SkeletalMeshComponent"))
  (if (Utilities|IsValid (Variables|Default|GetPlayerMesh))
    (CallFunction|ApplyMaterialOverlay :!label _label)
    (if (Utilities|Time|IsValidTimerHandle (Variables|Components|GetEffectTimer))
      (Utilities|Time|ClearandInvalidateTimerbyHandle (Variables|Components|GetEffectTimer)))
    (bind _returnvalue_3 (Utilities|Time|SetTimerbyFunctionName 0 "HandlingMaterialEffect" (Variables|MaterialParams|GetDuration)))
    (Variables|Components|SetEffectTimer _returnvalue_3)
    (else
      (Development|PrintString "There is no valid skeletal mesh set" true true "(R=1.000000,G=0.585570,B=0.000000,A=1.000000)")
      (if (Utilities|IsValid _returnvalue_2)
        (Variables|Default|SetPlayerMesh _returnvalue_2)
        (goto _label)
        (else
          (bind _returnvalue_4 (Game|AddComponentbyClass _returnvalue "/Script/Engine.SkeletalMeshComponent" false))
          (Components|SkeletalMesh|SetSkeletalMeshAsset _returnvalue_4 "/Game/ThirdPartyAssets/PolygonFantasyRivals/Meshes/Characters/SK_Character_Ancient_Warrior_01.SK_Character_Ancient_Warrior_01"))))))

(event Custom|ApplyMaterialOverlay
  (Rendering|Material|SetOverlayMaterial (Variables|Default|GetPlayerMesh) (Variables|Components|GetMaterialInstance) :!class /Script/Engine.MeshComponent))

(event Custom|ClearMaterialOverlay
  (bind _playermesh (Variables|Default|GetPlayerMesh))
  (if (Utilities|IsValid _playermesh)
    (Rendering|Material|SetOverlayMaterial _playermesh 0 :!class /Script/Engine.MeshComponent)))

(event EventBeginPlay
  (bind _returnvalue (Rendering|Material|CreateDynamicMaterialInstance "/Game/Materials/Characters/M_DamageOverlay.M_DamageOverlay" "None" "None" :!class /Script/Engine.KismetMaterialLibrary))
  (Variables|Components|SetMaterialInstance _returnvalue)
  (Material|ApplyMaterialDefaults)
  (Material|SetOpacity 0.0))

(event EventTick
  (params (DeltaSeconds :type Float%20%28single-precision%29))
  (Handling|HandlingMaterialEffect))

(fn HandlingMaterialEffect
  (bind _effecttimer (Variables|Components|GetEffectTimer))
  (if (Utilities|IsValid (Variables|Components|GetMaterialInstance))
    (if (not (Utilities|Time|IsTimerActivebyHandle _effecttimer))
      (Material|SetOpacity 0.0 :!label _label)
      (Utilities|Time|ClearandInvalidateTimerbyHandle (Variables|Components|GetEffectTimer))
      (else
        (Material|SetOpacity (* (Math|Float|Absolute(Float) (Math|Trig|Sin(Radians) (* (/ (Class|KismetSystemLibrary|GetTimerElapsedTimeHandle _effecttimer) (Variables|MaterialParams|GetDuration)) (Math|Trig|GetPI) (Variables|MaterialParams|GetCycles)))) (Variables|MaterialParams|GetOpacity)))
        (if (<= (Utilities|Time|GetTimerRemainingTimebyHandle (Variables|Components|GetEffectTimer)) 0.0)
          (goto _label))))))

(fn SetEmission
  (params (Value :type Float%20%28single-precision%29))
  (Rendering|Material|SetScalarParameterValue (Variables|Components|GetMaterialInstance) "EmissiveStrength" Value :!class /Script/Engine.MaterialInstanceDynamic))

(fn SetOpacity
  (params (Value :type Float%20%28single-precision%29))
  (Rendering|Material|SetScalarParameterValue (Variables|Components|GetMaterialInstance) "Opacity" Value :!class /Script/Engine.MaterialInstanceDynamic))

(fn SetColor
  (params (Value :type Linear%20Color%20Structure))
  (Rendering|Material|SetVectorParameterValue (Variables|Components|GetMaterialInstance) "Color" Value :!class /Script/Engine.MaterialInstanceDynamic))

(fn ApplyMaterialDefaults
  (Material|SetEmission (Variables|MaterialParams|GetEmission))
  (Material|SetColor (Variables|MaterialParams|GetColor)))

(fn SetPlayerMesh
  (params (PlayerMesh :type Skeletal%20Mesh%20Component%20Object%20Reference))
  (Variables|Default|SetPlayerMesh PlayerMesh))