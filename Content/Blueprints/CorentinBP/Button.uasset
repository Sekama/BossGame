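; Button actor that controls bridges when a player projectile hits it.
; An overlap of its Cube with an actor tagged PlayerProjectile calls DeployBridge on every valid entry in its Bridges array.
; It then searches the level for BridgeClosed actors whose TargetValue equals its ButtonValue, reverting them if Open is true and deploying them otherwise.
; The Open flag is only read here, never set.
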(event OnComponentBeginOverlap(Cube)
  (params (OverlappedComponent :type Primitive%20Component%20Object%20Reference) (OtherActor :type Actor%20Object%20Reference) (OtherComp :type Primitive%20Component%20Object%20Reference) (OtherBodyIndex :type Integer) (bFromSweep :type Boolean) (SweepResult :type Hit%20Result%20Structure%20%28by%20ref%29))
  (if (Actor|ActorHasTag OtherActor "PlayerProjectile")
    (Utilities|FlowControl|Sequence
      (:then_0
        (bind _array_element (Utilities|Array|ForEachLoopwithBreak (Variables|Default|GetBridges))
          (:LoopBody
            (Utilities|IsValid _array_element
              (:Is%20Valid
                (Default|DeployBridge _array_element))))))
      (:then_1
        (bind _outactors (Actor|GetAllActorsOfClass "/Game/Blueprints/CorentinBP/BridgeClosed.BridgeClosed_C"))
        (bind _array_element_2 (Utilities|Array|ForEachLoopwithBreak _outactors)
          (:LoopBody
            (Utilities|IsValid _array_element_2
              (:Is%20Valid
                (if (== (Variables|/Game/Blueprints/CorentinBP/BridgeClosed.BridgeClosed_C|GetTarget%20Value _array_element_2) (Variables|Default|GetButtonValue))
                  (if (Variables|Default|GetOpen?)
                    (Default|RevertBridge _array_element_2)
                    (else
                      (Default|DeployBridge _array_element_2))))))))))))

(event EventBeginPlay)

(event Collision|EventActorBeginOverlap
  (params (OtherActor :type Actor%20Object%20Reference)))

(event EventTick
  (params (DeltaSeconds :type Float%20%28single-precision%29)))

(fn ConstructionScript)