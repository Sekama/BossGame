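; BP_MasterCutscene is a cutscene controller actor that plays a level sequence alongside a dialogue window.
; BeginPlay creates the dialogue widget with UI-only input and, with AutoInit, plays the current entry in Sequencers, destroying itself if none exist.
; Exposed events update or show dialogue, pause the sequence while dialogue is active, and switch levels.
; The widget's continue press hides dialogue and resumes playback.
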(event Custom|InitSequence
  (bind _result (Utilities|Set|ToArray (Variables|Sequence|GetSequencers)))
  (if (Utilities|Array|IsNotEmpty _result)
    (bind _result_2 (Utilities|Set|ToArray (Variables|Sequence|GetSequencers)))
    (bind _output_get (Variables|Sequence|SetActiveSequencer (Utilities|Array|Get(acopy) _result_2 (Variables|Sequence|GetCurrentSequence))))
    (Sequencer|Player|Play (Variables|/Script/LevelSequence.LevelSequenceActor|GetSequencePlayer _output_get) :!class /Script/MovieScene.MovieSceneSequencePlayer)
    (else
      (Actor|DestroyActor))))

(event Custom|ContinueSequence
  (if (Variables|Default|GetDialogueActive?)
    (CallFunction|HideDialogue)
    (Sequencer|Player|Play (Variables|/Script/LevelSequence.LevelSequenceActor|GetSequencePlayer (Variables|Sequence|GetActiveSequencer)) :!class /Script/MovieScene.MovieSceneSequencePlayer)))

(event Custom|HideDialogue
  (Default|HideDialogueBox (Variables|Default|GetDialougeWidget) false)
  (Variables|Default|SetDialogueActive? false))

(event Custom|PauseSequence
  (if (Variables|Default|GetDialogueActive?)
    (Sequencer|Player|Pause (Variables|/Script/LevelSequence.LevelSequenceActor|GetSequencePlayer (Variables|Sequence|GetActiveSequencer)))))

(event Custom|SwitchScene
  (params (Level :type World%20Soft%20Object%20Reference))
  (Game|OpenLevel(byObjectReference) Level))

(event Custom|DisplayDialogue
  (Default|DisplayDialogueBox (Variables|Default|GetDialougeWidget))
  (Variables|Default|SetDialogueActive? true))

(event Custom|UpdateDialogue
  (params (Speaker :type String) (Message :type String))
  (Default|UpdateDialogue (Variables|Default|GetDialougeWidget) Speaker Message)
  (CallFunction|DisplayDialogue))

(event EventBeginPlay
  (bind _returnvalue (UserInterface|CreateWidget "/Game/UI/Widget_DialogueWindow.Widget_DialogueWindow_C" (Game|GetPlayerController 0)))
  (bind _output_get (Variables|Default|SetDialougeWidget _returnvalue))
  (UserInterface|Viewport|AddtoViewport _output_get 0)
  (Input|SetInputModeUIOnly (Game|GetPlayerController 0) _output_get "DoNotLock" false)
  (EventDispatchers|BindEventtoPressedtoContinue _output_get (delegate Custom|ContinueSequence))
  (if (Variables|Sequence|GetAutoInit?)
    (CallFunction|InitSequence)))

(event EventDestroyed
  (bind _dialougewidget (Variables|Default|GetDialougeWidget))
  (EventDispatchers|UnbindEventfromPressedtoContinue _dialougewidget (delegate Custom|ContinueSequence))
  (Widget|RemovefromParent _dialougewidget))

(event EventEndPlay
  (params (EndPlayReason :type EEndPlayReason%20Enum :default "Destroyed"))
  (bind _dialougewidget (Variables|Default|GetDialougeWidget))
  (EventDispatchers|UnbindEventfromPressedtoContinue _dialougewidget (delegate Custom|ContinueSequence))
  (Widget|RemovefromParent _dialougewidget))

(fn ConstructionScript)