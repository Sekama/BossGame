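; Laser turret hazard that, while active, sweeps a Niagara beam around the player and damages them when its end-point collision overlaps them.
; The beam end moves at constant speed to random offsets around and below the player, pausing briefly before retargeting, while yaw and pitch platforms track it.
; A player projectile hitting the sphere collision deactivates it, hiding its visuals, disabling collision, stopping sound and calling OnDisable.
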(event OnComponentBeginOverlap(SphereCollision)
  (params (OverlappedComponent :type Primitive%20Component%20Object%20Reference) (OtherActor :type Actor%20Object%20Reference) (OtherComp :type Primitive%20Component%20Object%20Reference) (OtherBodyIndex :type Integer) (bFromSweep :type Boolean) (SweepResult :type Hit%20Result%20Structure%20%28by%20ref%29))
  (if (Actor|ActorHasTag OtherActor "PlayerProjectile")
    (CallFunction|SetIsActive false)
    (Actor|DestroyActor OtherActor)))

(event OnComponentBeginOverlap(LaserCollision)
  (params (OverlappedComponent :type Primitive%20Component%20Object%20Reference) (OtherActor :type Actor%20Object%20Reference) (OtherComp :type Primitive%20Component%20Object%20Reference) (OtherBodyIndex :type Integer) (bFromSweep :type Boolean) (SweepResult :type Hit%20Result%20Structure%20%28by%20ref%29))
  (if (Actor|ActorHasTag OtherActor "Player")
    (bind _asbp_player (Utilities|Casting|CastToBP_Player OtherActor))
    (Class|HealthComponent|TakeDamage (Variables|/Script/GP4.PlayerCharacter|GetHealthComponent _asbp_player) 1.0 false)))

(event Custom|MoveTargetVector
  (bind _output_get (Variables|Default|SetCurrentVector (Math|Interpolation|VInterptoConstant (Variables|Default|GetCurrentVector) (Variables|Default|GetTargetVector) (Variables|Default|GetDeltaTime) (Variables|Default|GetInterp%20Speed))))
  (Effects|Components|ParticleSystem|SetVectorParameter (Variables|Default|GetNiagara) "Location" _output_get))

(event Custom|CheckDistance
  (if (< (Math|Vector|Distance(Vector) (Variables|Default|GetCurrentVector) (Variables|Default|GetTargetVector)) (Variables|Default|GetDistanceCheck))
    (if (not (Variables|Default|GetIsOnCooldown))
      (Variables|Default|SetStopTimer 0.0)
      (Variables|Default|SetIsOnCooldown true))))

(event Custom|CheckCooldown
  (if (Variables|Default|GetIsOnCooldown)
    (if (< (Variables|Default|GetStopTimer) (Variables|Default|GetMoveCooldown))
      (Variables|Default|SetStopTimer (+ (Variables|Default|GetStopTimer) (Variables|Default|GetDeltaTime)))
      (else
        (Variables|Default|SetIsOnCooldown false)
        (CallFunction|SetTargetVector)
        (Variables|Default|SetMoveCooldown (Math|Random|RandomFloatinRange 1.0 2.0))))))

(event Custom|SetIsActive
  (params (Activate? :type Boolean))
  (bind _output_get (Variables|Default|SetIsActivated Activate?))
  (if _output_get
    (Rendering|SetVisibility (Variables|Default|GetNiagara) true false)
    (Collision|SetCollisionEnabled (Variables|Default|GetSphereCollision) "QueryOnly")
    (Collision|SetCollisionEnabled (Variables|Default|GetLaserCollision) "QueryOnly")
    (Rendering|SetVisibility (Variables|Default|GetRunePlane) true false)
    (bind _returnvalue (Audio|SpawnSoundatLocation "/Game/Sounds/MetaSounds/TurretSound_MSS.TurretSound_MSS" (Variables|Default|GetTargetVector) "0, 0, 0" 1.0 1.0 0.0 0 0))
    (Variables|Default|SetSoundComp _returnvalue)
    (else
      (Rendering|SetVisibility (Variables|Default|GetNiagara) false false)
      (Collision|SetCollisionEnabled (Variables|Default|GetSphereCollision) "NoCollision")
      (Collision|SetCollisionEnabled (Variables|Default|GetLaserCollision) "NoCollision")
      (Rendering|SetVisibility (Variables|Default|GetRunePlane) false false)
      (Default|CallOnDisable)
      (Audio|Components|Audio|Stop (Variables|Default|GetSoundComp))
      (Components|DestroyComponent (Variables|Default|GetSoundComp)))))

(event Custom|Activate
  (CallFunction|SetIsActive true))

(event EventTick
  (params (DeltaSeconds :type Float%20%28single-precision%29))
  (bind _soundcomp (Variables|Default|GetSoundComp))
  (Variables|Default|SetDeltaTime DeltaSeconds)
  (if (Variables|Default|GetIsActivated)
    (CallFunction|RotateYaw)
    (CallFunction|RotatePitch)
    (CallFunction|CheckDistance)
    (CallFunction|MoveTargetVector)
    (CallFunction|CheckCooldown)
    (CallFunction|SetCollisionPosition)
    (Utilities|IsValid _soundcomp
      (:Is%20Valid
        (Transformation|SetRelativeLocation _soundcomp (Variables|Default|GetTargetVector) false false)))))

(event EventBeginPlay
  (bind _output_get (Variables|Default|SetTargetVector (Transformation|GetWorldLocation (Variables|Default|GetStartPosition))))
  (bind _output_get_2 (Variables|Default|SetCurrentVector _output_get))
  (Effects|Components|ParticleSystem|SetVectorParameter (Variables|Default|GetNiagara) "Location" _output_get_2))

(fn ConstructionScript)

(fn GetRandomXY
  (bind _maxrandomrangefromplayer (Variables|Default|GetMaxRandomRangeFromPlayer))
  (bind _maxrandomrangefromplayer_2 (Variables|Default|GetMaxRandomRangeFromPlayer))
  (bind _returnvalue (* _maxrandomrangefromplayer_2 -1.0))
  (bind _returnvalue_2 (Math|Random|RandomFloatinRange _returnvalue _maxrandomrangefromplayer))
  (return (Math|Vector|MakeVector _returnvalue_2 _returnvalue_2 -1e+02)))

(fn RotatePitch
  (Transformation|SetRelativeRotation (Variables|Default|GetPitchPlatform) (Math|Rotator|MakeRotator -9e+01 (* (.pitch (Math|Rotator|FindLookatRotation (Transformation|GetWorldLocation (Variables|Default|GetPitchPlatform)) (Variables|Default|GetCurrentVector))) -1.0) 0.0) false false))

(fn RotateYaw
  (Transformation|SetWorldRotation (Variables|Default|GetYawPlatform) (Math|Rotator|MakeRotator -1.8e+02 0.0 (.yaw (Math|Rotator|FindLookatRotation (Transformation|GetWorldLocation (Variables|Default|GetYawPlatform)) (Variables|Default|GetCurrentVector)))) false false))

(fn SetTargetVector
  (bind _randomxy (CallFunction|GetRandomXY))
  (Variables|Default|SetTargetVector (+ (Transformation|GetActorLocation (Game|Player|GetPlayerPawn 0)) _randomxy)))

(fn SetCollisionPosition
  (Transformation|SetWorldLocation (Variables|Default|GetLaserCollision) (Variables|Default|GetCurrentVector) false false))