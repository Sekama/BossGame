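; BP_BigSunBeam is a boss ability effect that plays a grow-and-shrink animation on its BPOrb component when spawned.
; BeginPlay calls Expand, where one timeline scales the orb from zero to full, then a two-second delay leads into a second timeline shrinking it to zero.
; Decrease restarts the grow timeline despite its name, and its only caller is disconnected leftover logic for animating light intensity and beam mesh scale.
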(event Custom|Expand
  (bind _bp_orb (Variables|Default|GetBP_Orb))
  (bind _newtrack_0 (Timeline|Timeline_1 PlayFromStart)
    (:Update
      (Transformation|SetRelativeScale3D _bp_orb (Math|Vector|MakeVector (Math|Float|Lerp 0.0 1.0 _newtrack_0) (Math|Float|Lerp 0.0 1.0 _newtrack_0) (Math|Float|Lerp 0.0 1.0 _newtrack_0))))
    (:Finished
      (Utilities|FlowControl|Delay 2.0)
      (bind _newtrack_0_2 (Timeline|Timeline_0 PlayFromStart)
        (:Update
          (Transformation|SetRelativeScale3D _bp_orb (Math|Vector|MakeVector (Math|Float|Lerp 1.0 0.0 _newtrack_0_2) (Math|Float|Lerp 1.0 0.0 _newtrack_0_2) (Math|Float|Lerp 1.0 0.0 _newtrack_0_2))))))))

(event Custom|Decrease
  (bind _bp_orb (Variables|Default|GetBP_Orb))
  (bind _newtrack_0 (Timeline|Timeline_1 PlayFromStart)
    (:Update
      (Transformation|SetRelativeScale3D _bp_orb (Math|Vector|MakeVector (Math|Float|Lerp 0.0 1.0 _newtrack_0) (Math|Float|Lerp 0.0 1.0 _newtrack_0) (Math|Float|Lerp 0.0 1.0 _newtrack_0))))
    (:Finished
      (Utilities|FlowControl|Delay 2.0)
      (bind _newtrack_0_2 (Timeline|Timeline_0 PlayFromStart)
        (:Update
          (Transformation|SetRelativeScale3D _bp_orb (Math|Vector|MakeVector (Math|Float|Lerp 1.0 0.0 _newtrack_0_2) (Math|Float|Lerp 1.0 0.0 _newtrack_0_2) (Math|Float|Lerp 1.0 0.0 _newtrack_0_2))))))))

(event EventBeginPlay
  (CallFunction|Expand))

(event EventTick
  (params (DeltaSeconds :type Float%20%28single-precision%29)))

(fn ConstructionScript)