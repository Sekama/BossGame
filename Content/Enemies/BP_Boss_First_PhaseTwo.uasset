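; Second-phase first boss, driven by a Blackboard BossPhase value, with monolith, minion and shockwave attack events.
; StartPhaseTwo sets BossPhase to 1; once every activated monolith reports disabled, it becomes 3 and Tick smoothly yaws the boss toward the player.
; Callable events spawn minions at offsets and shockwaves at left or right slam points.
; Player projectiles overlapping the Target component damage HealthComponent, whose death event reloads the current level.
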(event OnComponentBeginOverlap(Target)
  (params (OverlappedComponent :type Primitive%20Component%20Object%20Reference) (OtherActor :type Actor%20Object%20Reference) (OtherComp :type Primitive%20Component%20Object%20Reference) (OtherBodyIndex :type Integer) (bFromSweep :type Boolean) (SweepResult :type Hit%20Result%20Structure%20%28by%20ref%29))
  (if (Actor|ActorHasTag OtherActor "PlayerProjectile")
    (Class|HealthComponent|TakeDamage (Variables|Default|GetHealthComponent) 1.0 false)))

(event OnDeath(HealthComponent)
  (bind _returnvalue (Game|GetCurrentLevelName true))
  (Game|OpenLevel(byName) (Utilities|String|StringToName _returnvalue)))

(event Custom|ActivateMonoliths
  (if (not (Variables|Default|GetIsMonolithsActive?))
    (Variables|Default|SetIsMonolithsActive? true)
    (for _array_element (Variables|Default|GetMonoliths)
      (Default|Activate _array_element))))

(event Custom|OnAllMonolithsDisabled
  (bind _returnvalue (AI|GetBlackboard 0))
  (Class|BlackboardComponent|SetValueasInt _returnvalue (Utilities|Name|MakeLiteralName "BossPhase") 3)
  (AI|Components|Blackboard|SetValueasBool _returnvalue (Utilities|Name|MakeLiteralName "IsMonolithsActive?") false)
  (Variables|Default|SetIsMonolithsActive? false))

(event Custom|OnDisableMonolith
  (bind _result (Math|Integer|IncrementInt (Variables|Default|GetMonolithsDisabled))
    (:%20%20
      (if (>= _result (Utilities|Array|Length (Variables|Default|GetMonoliths)))
        (CallFunction|OnAllMonolithsDisabled)
        (Variables|Default|SetMonolithsDisabled 0)))))

(event Custom|StartPhaseTwo
  (Class|BlackboardComponent|SetValueasInt (AI|GetBlackboard 0) (Utilities|Name|MakeLiteralName "BossPhase") 1))

(event Custom|SpawnMinions
  (for _array_element (Variables|Default|GetMinionSpawnLocations)
    (Game|SpawnActorfromClass "/Game/Enemies/BP_PhaseTwoMinion.BP_PhaseTwoMinion_C" (Math|Transform|MakeTransform (+ (Transformation|GetActorLocation) _array_element) "0, 0, 0" "1.000000,1.000000,1.000000") "AlwaysSpawn" 0 0)))

(event Custom|RotateToPlayer
  (bind _returnvalue (Transformation|GetActorRotation))
  (bind _returnvalue_2 (Transformation|GetActorRotation))
  (bind _returnvalue_3 (Transformation|GetActorLocation))
  (bind _as_bp_player (Variables|Default|GetAs%20BP%20Player))
  (bind _rotationinterp_speed (Variables|Default|GetRotationInterp%20Speed))
  (bind _delta_seconds (Variables|Default|GetDelta%20Seconds))
  (bind _returnvalue_4 (Transformation|GetActorLocation _as_bp_player))
  (bind _returnvalue_5 (Math|Rotator|FindLookatRotation _returnvalue_3 _returnvalue_4))
  (bind _returnvalue_6 (Class|KismetMathLibrary|RInterptoConstant _returnvalue_2 (Math|Rotator|MakeRotator (.roll _returnvalue) (.pitch _returnvalue) (.yaw _returnvalue_5)) _delta_seconds _rotationinterp_speed))
  ;[1 1 1] RotateToPlayer
  (Transformation|SetActorRotation (Math|Rotator|MakeRotator (.roll _returnvalue_6) (.pitch _returnvalue_6) (.yaw _returnvalue_6))))

(event Custom|Init
  (bind _asbp_player (Utilities|Casting|CastToBP_Player (Game|Player|GetPlayerPawn 0)))
  (Variables|Default|SetAs%20BP%20Player _asbp_player)
  (for _array_element (Variables|Default|GetMonoliths)
    (EventDispatchers|BindEventtoOnDisable _array_element (delegate Custom|OnDisableMonolith))))

(event Custom|PlayShockwaveRight
  (Game|SpawnActorfromClass "/Game/Enemies/BP_ShockwaveActor.BP_ShockwaveActor_C" (Math|Transform|MakeTransform (Transformation|GetWorldLocation (Variables|Default|GetSlamLocationRight)) "0, 0, 0" "1.000000,1.000000,1.000000") "AlwaysSpawn" 0 0))

(event Custom|PlayShockwaveLeft
  (Game|SpawnActorfromClass "/Game/Enemies/BP_ShockwaveActor.BP_ShockwaveActor_C" (Math|Transform|MakeTransform (Transformation|GetWorldLocation (Variables|Default|GetSlamLocationLeft)) "0, 0, 0" "1.000000,1.000000,1.000000") "AlwaysSpawn" 0 0))

(event EventTick
  (params (DeltaSeconds :type Float%20%28single-precision%29))
  (Variables|Default|SetDelta%20Seconds DeltaSeconds)
  (if (== (Class|BlackboardComponent|GetValueasInt (AI|GetBlackboard 0) (Utilities|Name|MakeLiteralName "BossPhase")) 3)
    (CallFunction|RotatetoPlayer)))

(event EventBeginPlay
  (CallFunction|Init))

(fn ConstructionScript)