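; BP_Boss_Second is a boss enemy whose Eye component is the hit zone for player projectiles.
; Overlaps from actors tagged PlayerProjectile deal one point of non-critical damage through the HealthComponent, print the remaining health and destroy the projectile.
; When the HealthComponent fires OnDeath, the current level is reopened by name.
; BeginPlay caches a cast reference to the player pawn, which the graph does not otherwise use.
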(event OnComponentBeginOverlap(Eye)
  (params (OverlappedComponent :type Primitive%20Component%20Object%20Reference) (OtherActor :type Actor%20Object%20Reference) (OtherComp :type Primitive%20Component%20Object%20Reference) (OtherBodyIndex :type Integer) (bFromSweep :type Boolean) (SweepResult :type Hit%20Result%20Structure%20%28by%20ref%29))
  (if (Actor|ActorHasTag OtherActor "PlayerProjectile")
    (Class|HealthComponent|TakeDamage (Variables|Default|GetHealthComponent) 1.0 false)
    (Development|PrintString (Utilities|String|ToString(Float) (Variables|/Script/GP4.HealthComponent|GetCurrentHealth (Variables|Default|GetHealthComponent))))
    (Actor|DestroyActor OtherActor)))

(event OnDeath(HealthComponent)
  (bind _returnvalue (Game|GetCurrentLevelName true))
  (Game|OpenLevel(byName) (Utilities|String|StringToName _returnvalue)))

(event EventBeginPlay
  (bind _asbp_player (Utilities|Casting|CastToBP_Player (Game|Player|GetPlayerPawn 0)))
  (Variables|Default|SetAs%20BP%20Player _asbp_player))

(fn ConstructionScript)