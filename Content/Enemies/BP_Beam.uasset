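; BP_Beam is an enemy beam hazard that periodically damages the player standing inside it and removes itself after about ten seconds.
; CollisionBox overlap events toggle a TakeDamage flag for actors tagged Player.
; Delay nodes on Tick act as timers: one destroys the actor, the other checks the flag roughly every second and damages player 0's HealthComponent.
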(event OnComponentBeginOverlap(CollisionBox)
  (params (OverlappedComponent :type Primitive%20Component%20Object%20Reference) (OtherActor :type Actor%20Object%20Reference) (OtherComp :type Primitive%20Component%20Object%20Reference) (OtherBodyIndex :type Integer) (bFromSweep :type Boolean) (SweepResult :type Hit%20Result%20Structure%20%28by%20ref%29))
  (if (Actor|ActorHasTag OtherActor "Player")
    (Variables|Default|SetTakeDamage true)))

(event OnComponentEndOverlap(CollisionBox)
  (params (OverlappedComponent :type Primitive%20Component%20Object%20Reference) (OtherActor :type Actor%20Object%20Reference) (OtherComp :type Primitive%20Component%20Object%20Reference) (OtherBodyIndex :type Integer))
  (if (Actor|ActorHasTag OtherActor "Player")
    (Variables|Default|SetTakeDamage false)))

(event EventTick
  (params (DeltaSeconds :type Float%20%28single-precision%29))
  (Utilities|FlowControl|Sequence
    (:then_0
      (Utilities|FlowControl|Delay 1e+01)
      (Actor|DestroyActor))
    (:then_1
      (Utilities|FlowControl|Delay 1.0)
      (if (Variables|Default|GetTakeDamage)
        (bind _asbp_player (Utilities|Casting|CastToBP_Player (Game|Player|GetPlayerPawn 0)))
        (Class|HealthComponent|TakeDamage (Variables|/Script/GP4.PlayerCharacter|GetHealthComponent _asbp_player) 1.0 false)))))

(fn ConstructionScript)