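; First boss enemy, apparently a golem, kept in a deprecated folder; it damages the player on contact and dies to player projectiles.
; Every Tick it calls UseBlackboard on BB_Boss and copies CanWalk from Golem_Anim_BP into the blackboard.
; AtColBox tracks PInRange, which Sphere_L also clears on exit after dealing damage on entry.
; Tagged projectiles hitting Target damage its HealthComponent, whose OnDeath destroys the actor.
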(event OnComponentBeginOverlap(AtColBox)
  (params (OverlappedComponent :type Primitive%20Component%20Object%20Reference) (OtherActor :type Actor%20Object%20Reference) (OtherComp :type Primitive%20Component%20Object%20Reference) (OtherBodyIndex :type Integer) (bFromSweep :type Boolean) (SweepResult :type Hit%20Result%20Structure%20%28by%20ref%29))
  (Utilities|Casting|CastToBP_Player OtherActor)
  (Variables|Default|SetpInRange true))

(event OnComponentEndOverlap(AtColBox)
  (params (OverlappedComponent :type Primitive%20Component%20Object%20Reference) (OtherActor :type Actor%20Object%20Reference) (OtherComp :type Primitive%20Component%20Object%20Reference) (OtherBodyIndex :type Integer))
  (Utilities|Casting|CastToBP_Player OtherActor)
  (Variables|Default|SetpInRange false))

(event OnDeath(HealthComponent)
  (Actor|DestroyActor))

(event OnComponentBeginOverlap(Target)
  (params (OverlappedComponent :type Primitive%20Component%20Object%20Reference) (OtherActor :type Actor%20Object%20Reference) (OtherComp :type Primitive%20Component%20Object%20Reference) (OtherBodyIndex :type Integer) (bFromSweep :type Boolean) (SweepResult :type Hit%20Result%20Structure%20%28by%20ref%29))
  (if (Actor|ActorHasTag OtherActor "PlayerProjectile")
    (Class|HealthComponent|TakeDamage (Variables|Default|GetHealthComponent) 1.0 false)))

(event OnComponentBeginOverlap(Sphere_L)
  (params (OverlappedComponent :type Primitive%20Component%20Object%20Reference) (OtherActor :type Actor%20Object%20Reference) (OtherComp :type Primitive%20Component%20Object%20Reference) (OtherBodyIndex :type Integer) (bFromSweep :type Boolean) (SweepResult :type Hit%20Result%20Structure%20%28by%20ref%29))
  (bind _asbp_player (Utilities|Casting|CastToBP_Player OtherActor))
  (Class|HealthComponent|TakeDamage (Variables|/Script/GP4.PlayerCharacter|GetHealthComponent _asbp_player) 1.0 false))

(event OnComponentEndOverlap(Sphere_L)
  (params (OverlappedComponent :type Primitive%20Component%20Object%20Reference) (OtherActor :type Actor%20Object%20Reference) (OtherComp :type Primitive%20Component%20Object%20Reference) (OtherBodyIndex :type Integer))
  (Utilities|Casting|CastToBP_Player OtherActor)
  (Variables|Default|SetpInRange false))

(event EventBeginPlay)

(event Collision|EventActorBeginOverlap
  (params (OtherActor :type Actor%20Object%20Reference)))

(event EventTick
  (params (DeltaSeconds :type Float%20%28single-precision%29))
  (Utilities|FlowControl|Sequence
    (:then_0
      (bind _asgolem_anim_bp (Utilities|Casting|CastToGolem_Anim_BP (Components|SkeletalMesh|GetAnimInstance (Variables|Character|GetMesh))))
      (bind _blackboardcomponent (Class|AIController|UseBlackboard (AI|GetAIController (Pawn|GetController)) "/Game/Enemies/BehaviorTrees/BB_Boss.BB_Boss"))
      (AI|Components|Blackboard|SetValueasBool _blackboardcomponent (Utilities|Name|MakeLiteralName "CanWalk?") (Variables|/Game/Enemies/Golem_Anim_BP.Golem_Anim_BP_C|GetCan%20walk _asgolem_anim_bp)))))

(fn ConstructionScript)