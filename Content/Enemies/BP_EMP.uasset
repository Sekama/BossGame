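; BP_EMP is an enemy EMP effect actor that shows an expanding shockwave.
; Each Tick it grows the ShockWave component uniformly toward MaxSize using constant-speed interpolation of its world scale.
; The actor destroys itself once the scale reaches MaxSize.
; Its overlap event is empty, so the file applies no effect to anything the wave touches.
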(event Custom|Increase
  (params (DeltaTIme :type Float%20%28double-precision%29))
  (bind _shockwave (Variables|Default|GetShockWave))
  (bind _maxsize (Variables|Default|GetMaxSize))
  (bind _returnvalue (Transformation|GetWorldScale _shockwave))
  (bind _returnvalue_2 (Math|Interpolation|FInterptoConstant (.x _returnvalue) _maxsize DeltaTIme 3e+01))
  (Transformation|SetWorldScale3D _shockwave (Math|Vector|MakeVector _returnvalue_2 _returnvalue_2 _returnvalue_2))
  (if (>= (.x _returnvalue) _maxsize)
    (Actor|DestroyActor)))

(event Collision|EventActorBeginOverlap
  (params (OtherActor :type Actor%20Object%20Reference)))

(event EventTick
  (params (DeltaSeconds :type Float%20%28single-precision%29))
  (CallFunction|Increase DeltaSeconds))

(fn ConstructionScript)