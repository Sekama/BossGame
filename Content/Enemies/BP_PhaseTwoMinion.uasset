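; BP_PhaseTwoMinion is an enemy minion that dies on its first contact with a player projectile or the player.
; Its Sphere overlap handles actors tagged PlayerProjectile, damaging its own HealthComponent, then destroying itself and the projectile regardless of remaining health.
; Its capsule overlap handles actors tagged Player, damaging the BP_Player HealthComponent before destroying the minion.
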(event OnComponentBeginOverlap(CapsuleComponent)
  (params (OverlappedComponent :type Primitive%20Component%20Object%20Reference) (OtherActor :type Actor%20Object%20Reference) (OtherComp :type Primitive%20Component%20Object%20Reference) (OtherBodyIndex :type Integer) (bFromSweep :type Boolean) (SweepResult :type Hit%20Result%20Structure%20%28by%20ref%29))
  (if (Actor|ActorHasTag OtherActor "Player")
    (bind _asbp_player (Utilities|Casting|CastToBP_Player OtherActor))
    (Class|HealthComponent|TakeDamage (Variables|/Script/GP4.PlayerCharacter|GetHealthComponent _asbp_player) 1.0 false)
    (Actor|DestroyActor)))

(event OnComponentBeginOverlap(Sphere)
  (params (OverlappedComponent :type Primitive%20Component%20Object%20Reference) (OtherActor :type Actor%20Object%20Reference) (OtherComp :type Primitive%20Component%20Object%20Reference) (OtherBodyIndex :type Integer) (bFromSweep :type Boolean) (SweepResult :type Hit%20Result%20Structure%20%28by%20ref%29))
  (if (Actor|ActorHasTag OtherActor "PlayerProjectile")
    (Class|HealthComponent|TakeDamage (Variables|Default|GetHealthComponent) 1.0 false)
    (Actor|DestroyActor)
    (Actor|DestroyActor OtherActor)))

(fn ConstructionScript)