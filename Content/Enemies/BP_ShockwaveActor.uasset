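; Expanding shockwave hazard actor that damages the player it sweeps over.
; Each tick it grows the ShockWave component uniformly at a constant rate toward MaxSize, then destroys itself once that size is reached.
; When the component begins overlapping a BP_Player, it applies a small non-critical hit through that player's HealthComponent.
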(event OnComponentBeginOverlap(ShockWave)
  (params (OverlappedComponent :type Primitive%20Component%20Object%20Reference) (OtherActor :type Actor%20Object%20Reference) (OtherComp :type Primitive%20Component%20Object%20Reference) (OtherBodyIndex :type Integer) (bFromSweep :type Boolean) (SweepResult :type Hit%20Result%20Structure%20%28by%20ref%29))
  (bind _asbp_player (Utilities|Casting|CastToBP_Player OtherActor))
  (Class|HealthComponent|TakeDamage (Variables|/Script/GP4.PlayerCharacter|GetHealthComponent _asbp_player) 1.0 false))

(event Custom|Increase
  (params (DeltaTIme :type Float%20%28double-precision%29))
  (bind _shockwave (Variables|Default|GetShockWave))
  (bind _maxsize (Variables|Default|GetMaxSize))
  (bind _returnvalue (Transformation|GetWorldScale _shockwave))
  (bind _returnvalue_2 (Math|Interpolation|FInterptoConstant (.x _returnvalue) _maxsize DeltaTIme 15.0))
  (Transformation|SetWorldScale3D _shockwave (Math|Vector|MakeVector _returnvalue_2 _returnvalue_2 _returnvalue_2))
  (if (>= (.x _returnvalue) _maxsize)
    (Actor|DestroyActor)))

(event Collision|EventActorBeginOverlap
  (params (OtherActor :type Actor%20Object%20Reference)))

(event EventTick
  (params (DeltaSeconds :type Float%20%28single-precision%29))
  (CallFunction|Increase DeltaSeconds))

(fn ConstructionScript)