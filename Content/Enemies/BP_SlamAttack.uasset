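; Enemy slam attack actor that raises eight meshes in a staggered wave, damages the player on overlap, then destroys itself.
; BeginPlay fires one custom event per mesh at short intervals, each driving relative Z through its own timeline.
; Overlaps with Player-tagged actors deal damage through the HealthComponent of player pawn 0.
; MoveRock and MoveRock2 are alternative movement events that nothing here calls.
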(event Custom|Overlap
  (params (OverlappedComponent :type Primitive%20Component%20Object%20Reference) (OtherActor :type Actor%20Object%20Reference) (OtherComp :type Primitive%20Component%20Object%20Reference) (OtherBodyIndex :type Integer) (bFromSweep :type Boolean) (SweepResult :type Hit%20Result%20Structure%20%28by%20ref%29))
  (if (Actor|ActorHasTag OtherActor "Player")
    (bind _asbp_player (Utilities|Casting|CastToBP_Player (Game|Player|GetPlayerPawn 0)))
    (Class|HealthComponent|TakeDamage (Variables|/Script/GP4.PlayerCharacter|GetHealthComponent _asbp_player) 1.0 false)))

(event Custom|MoveRock
  (params (NewParam :type Static%20Mesh%20Component%20Object%20Reference))
  (bind _4 (Variables|Default|Get4))
  (bind _5 (Variables|Default|Get5))
  (bind _6 (Variables|Default|Get6))
  (bind _7 (Variables|Default|Get7))
  (bind _8 (Variables|Default|Get8))
  (bind _relativelocation (Variables|/Script/Engine.SceneComponent|GetRelativeLocation NewParam))
  (bind _2 (Variables|Default|Get2))
  (bind _3 (Variables|Default|Get3))
  (bind _relativelocation_2 (Variables|/Script/Engine.SceneComponent|GetRelativeLocation _4))
  (bind _relativelocation_3 (Variables|/Script/Engine.SceneComponent|GetRelativeLocation _5))
  (bind _relativelocation_4 (Variables|/Script/Engine.SceneComponent|GetRelativeLocation _6))
  (bind _relativelocation_5 (Variables|/Script/Engine.SceneComponent|GetRelativeLocation _7))
  (bind _relativelocation_6 (Variables|/Script/Engine.SceneComponent|GetRelativeLocation _8))
  (bind _relativelocation_7 (Variables|/Script/Engine.SceneComponent|GetRelativeLocation _2))
  (bind _relativelocation_8 (Variables|/Script/Engine.SceneComponent|GetRelativeLocation _3))
  (bind (_direction _upanddown _second _third _fourth _fifth _sixth _seventh _eighth) (Timeline|Timeline SetNewTime)
    (:Update
      (Transformation|SetRelativeLocation NewParam (Math|Vector|MakeVector (.x _relativelocation) (.y _relativelocation) _upanddown) false false)
      (Transformation|SetRelativeLocation _2 (Math|Vector|MakeVector (.x _relativelocation_7) (.y _relativelocation_7) _second) false false)
      (Transformation|SetRelativeLocation _3 (Math|Vector|MakeVector (.x _relativelocation_8) (.y _relativelocation_8) _third) false false)
      (Transformation|SetRelativeLocation _4 (Math|Vector|MakeVector (.x _relativelocation_2) (.y _relativelocation_2) _fourth) false false)
      (Transformation|SetRelativeLocation _5 (Math|Vector|MakeVector (.x _relativelocation_3) (.y _relativelocation_3) _fifth) false false)
      (Transformation|SetRelativeLocation _6 (Math|Vector|MakeVector (.x _relativelocation_4) (.y _relativelocation_4) _sixth) false false)
      (Transformation|SetRelativeLocation _7 (Math|Vector|MakeVector (.x _relativelocation_5) (.y _relativelocation_5) _seventh) false false)
      (Transformation|SetRelativeLocation _8 (Math|Vector|MakeVector (.x _relativelocation_6) (.y _relativelocation_6) _eighth) false false))
    (:Finished
      (Actor|DestroyActor))))

(event Custom|Mesh1
  (params (Mesh :type Static%20Mesh%20Component%20Object%20Reference))
  (bind _relativelocation (Variables|/Script/Engine.SceneComponent|GetRelativeLocation Mesh))
  (bind _upanddown (Timeline|Timeline_2 PlayFromStart)
    (:Update
      (Transformation|SetRelativeLocation Mesh (Math|Vector|MakeVector (.x _relativelocation) (.y _relativelocation) _upanddown) false false))))

(event Custom|Mesh2
  (params (Mesh :type Static%20Mesh%20Component%20Object%20Reference))
  (bind _relativelocation (Variables|/Script/Engine.SceneComponent|GetRelativeLocation Mesh))
  (bind _upanddown (Timeline|Timeline_3 PlayFromStart)
    (:Update
      (Transformation|SetRelativeLocation Mesh (Math|Vector|MakeVector (.x _relativelocation) (.y _relativelocation) _upanddown) false false))))

(event Custom|Mesh3
  (params (Mesh :type Static%20Mesh%20Component%20Object%20Reference))
  (bind _relativelocation (Variables|/Script/Engine.SceneComponent|GetRelativeLocation Mesh))
  (bind _upanddown (Timeline|Timeline_4 PlayFromStart)
    (:Update
      (Transformation|SetRelativeLocation Mesh (Math|Vector|MakeVector (.x _relativelocation) (.y _relativelocation) _upanddown) false false))))

(event Custom|Mesh4
  (params (Mesh :type Static%20Mesh%20Component%20Object%20Reference))
  (bind _relativelocation (Variables|/Script/Engine.SceneComponent|GetRelativeLocation Mesh))
  (bind _upanddown (Timeline|Timeline_5 PlayFromStart)
    (:Update
      (Transformation|SetRelativeLocation Mesh (Math|Vector|MakeVector (.x _relativelocation) (.y _relativelocation) _upanddown) false false))))

(event Custom|Mesh5
  (params (Mesh :type Static%20Mesh%20Component%20Object%20Reference))
  (bind _relativelocation (Variables|/Script/Engine.SceneComponent|GetRelativeLocation Mesh))
  (bind _upanddown (Timeline|Timeline_6 PlayFromStart)
    (:Update
      (Transformation|SetRelativeLocation Mesh (Math|Vector|MakeVector (.x _relativelocation) (.y _relativelocation) _upanddown) false false))))

(event Custom|Mesh6
  (params (Mesh :type Static%20Mesh%20Component%20Object%20Reference))
  (bind _relativelocation (Variables|/Script/Engine.SceneComponent|GetRelativeLocation Mesh))
  (bind _upanddown (Timeline|Timeline_1 PlayFromStart)
    (:Update
      (Transformation|SetRelativeLocation Mesh (Math|Vector|MakeVector (.x _relativelocation) (.y _relativelocation) _upanddown) false false))))

(event Custom|Mesh7
  (params (Mesh :type Static%20Mesh%20Component%20Object%20Reference))
  (bind _relativelocation (Variables|/Script/Engine.SceneComponent|GetRelativeLocation Mesh))
  (bind _upanddown (Timeline|Timeline_7 PlayFromStart)
    (:Update
      (Transformation|SetRelativeLocation Mesh (Math|Vector|MakeVector (.x _relativelocation) (.y _relativelocation) _upanddown) false false))))

(event Custom|MoveRock2
  (params (Mesh :type Static%20Mesh%20Component%20Object%20Reference))
  (bind _relativelocation (Variables|/Script/Engine.SceneComponent|GetRelativeLocation Mesh))
  (bind _upanddown (Timeline|Timeline_0 PlayFromStart)
    (:Update
      (Transformation|SetRelativeLocation Mesh (Math|Vector|MakeVector (.x _relativelocation) (.y _relativelocation) _upanddown) false false))))

(event Custom|Mesh8
  (params (Mesh :type Static%20Mesh%20Component%20Object%20Reference))
  (bind _relativelocation (Variables|/Script/Engine.SceneComponent|GetRelativeLocation Mesh))
  (bind _upanddown (Timeline|Timeline_8 PlayFromStart)
    (:Update
      (Transformation|SetRelativeLocation Mesh (Math|Vector|MakeVector (.x _relativelocation) (.y _relativelocation) _upanddown) false false))))

(event EventBeginPlay
  (Variables|Default|SetMeshArray (Utilities|Array|MakeArray (Variables|Default|Get1) (Variables|Default|Get2) (Variables|Default|Get3) (Variables|Default|Get4) (Variables|Default|Get5) (Variables|Default|Get6) (Variables|Default|Get8) (Variables|Default|Get7)))
  (Collision|BindEventtoOnComponentBeginOverlap (Variables|Default|GetMeshArray) (delegate Custom|Overlap))
  (CallFunction|Mesh1 (Variables|Default|Get1))
  (Utilities|FlowControl|Delay 0.2)
  (CallFunction|Mesh2 (Variables|Default|Get2))
  (Utilities|FlowControl|Delay 0.2)
  (CallFunction|Mesh3 (Variables|Default|Get3))
  (Utilities|FlowControl|Delay 0.2)
  (CallFunction|Mesh4 (Variables|Default|Get4))
  (Utilities|FlowControl|Delay 0.2)
  (CallFunction|Mesh5 (Variables|Default|Get5))
  (Utilities|FlowControl|Delay 0.2)
  (CallFunction|Mesh6 (Variables|Default|Get6))
  (Utilities|FlowControl|Delay 0.2)
  (CallFunction|Mesh7 (Variables|Default|Get7))
  (Utilities|FlowControl|Delay 0.2)
  (CallFunction|Mesh8 (Variables|Default|Get8))
  (Utilities|FlowControl|Delay 1.0)
  (Actor|DestroyActor))

(event EventTick
  (params (DeltaSeconds :type Float%20%28single-precision%29))
  (Variables|Default|SetDeltaTime DeltaSeconds))

(fn ConstructionScript)