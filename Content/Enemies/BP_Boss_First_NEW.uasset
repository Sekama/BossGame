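; First-phase golem boss that stomps out shockwaves, tracks the player with laser eye beams and starts phase two through the game mode on death.
; Tick relays walk, stomp, stagger and target-hit state between the actor, its anim blueprint and the BB_Boss blackboard.
; EMP hits stagger it and expose a rune weak point that takes heavy projectile damage until three hits hide it.
; Damage updates a boss health widget, with a delayed second value.
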(event OnComponentBeginOverlap(AtColBox)
  (params (OverlappedComponent :type Primitive%20Component%20Object%20Reference) (OtherActor :type Actor%20Object%20Reference) (OtherComp :type Primitive%20Component%20Object%20Reference) (OtherBodyIndex :type Integer) (bFromSweep :type Boolean) (SweepResult :type Hit%20Result%20Structure%20%28by%20ref%29))
  (Utilities|Casting|CastToBP_Player OtherActor)
  (Variables|Default|SetpInRange true))

(event OnComponentEndOverlap(AtColBox)
  (params (OverlappedComponent :type Primitive%20Component%20Object%20Reference) (OtherActor :type Actor%20Object%20Reference) (OtherComp :type Primitive%20Component%20Object%20Reference) (OtherBodyIndex :type Integer))
  (Utilities|Casting|CastToBP_Player OtherActor)
  (Variables|Default|SetpInRange false))

(event OnDeath(HealthComponent)
  (Components|DestroyComponent (Variables|Default|GetRuneMat))
  (Widget|RemovefromParent (Variables|Default|GetBossBarWidget))
  (Variables|Default|SetStaggered? false)
  (bind _blackboardcomponent (Class|AIController|UseBlackboard (AI|GetAIController (Pawn|GetController)) "/Game/Enemies/BehaviorTrees/BB_Boss.BB_Boss"))
  (AI|Components|Blackboard|SetValueasBool _blackboardcomponent (Utilities|Name|MakeLiteralName "isDead?") true)
  (Utilities|FlowControl|Delay 3.0)
  (bind _asbp_game_mode (Utilities|Casting|CastToBP_GameMode (Game|GetGameMode)))
  (Default|InitializePhase2 _asbp_game_mode))

(event OnComponentBeginOverlap(CapsuleComponent)
  (params (OverlappedComponent :type Primitive%20Component%20Object%20Reference) (OtherActor :type Actor%20Object%20Reference) (OtherComp :type Primitive%20Component%20Object%20Reference) (OtherBodyIndex :type Integer) (bFromSweep :type Boolean) (SweepResult :type Hit%20Result%20Structure%20%28by%20ref%29))
  (bind _target2 (Variables|Default|GetTarget2))
  (bind _healthcomponent (Variables|Default|GetHealthComponent))
  (if (Actor|ActorHasTag OtherActor "EMP")
    (Class|HealthComponent|TakeDamage _healthcomponent 2.0 false)
    (CallFunction|HealthBar)
    (Variables|Default|SetStaggered? true)
    (Utilities|FlowControl|Delay 2.0)
    (Collision|SetCollisionEnabled _target2 "QueryOnly")
    (Rendering|ToggleVisibility _target2 false)
    (elif (Actor|ActorHasTag OtherActor "PlayerProjectile")
      (Class|HealthComponent|TakeDamage _healthcomponent 1.0 false)
      (CallFunction|HealthBar))))

(event OnComponentBeginOverlap(Target2)
  (params (OverlappedComponent :type Primitive%20Component%20Object%20Reference) (OtherActor :type Actor%20Object%20Reference) (OtherComp :type Primitive%20Component%20Object%20Reference) (OtherBodyIndex :type Integer) (bFromSweep :type Boolean) (SweepResult :type Hit%20Result%20Structure%20%28by%20ref%29))
  (CallFunction|HurtTarget OtherActor)
  (Audio|PlaySoundatLocation "/Game/Sounds/WavAssets/SFX/Game/Splode07.Splode07" (Transformation|GetWorldLocation OverlappedComponent) "0, 0, 0" 1.0 1.0 0.0 0 0 0 0))

(event Custom|SetLaserEyeBeamEndLocation
  (bind _returnvalue (Game|Player|GetPlayerPawn 0))
  (bind _returnvalue_2 (Transformation|GetActorLocation _returnvalue))
  (Effects|Components|ParticleSystem|SetVectorParameter (Variables|Default|GetNE_LaserEyeBeam_Left) "Location" _returnvalue_2)
  (Effects|Components|ParticleSystem|SetVectorParameter (Variables|Default|GetNE_LaserEyeBeam_Right) "Location" _returnvalue_2))

(event Custom|SetStompAnimation
  (bind _asgolem_anim_bp (Utilities|Casting|CastToGolem_Anim_BP (Components|SkeletalMesh|GetAnimInstance (Variables|Character|GetMesh))))
  (Variables|/Game/Enemies/Golem_Anim_BP.Golem_Anim_BP_C|SetStomp? _asgolem_anim_bp (Variables|Default|Getstomp_Anim)))

(event Custom|STOMP
  (Utilities|FlowControl|Sequence
    (:then_0
      (Class|BossFirst|ActivateCollider)
      (Utilities|FlowControl|Delay 3.0)
      (Variables|Default|Setstomp_Anim false))
    (:then_1
      (Game|SpawnActorfromClass "/Game/Enemies/BP_ShockwaveActor.BP_ShockwaveActor_C" (Math|Conversions|ToTransform(Vector) (.location (Transformation|GetSocketTransform (Variables|Character|GetMesh) "Foot_L" "RTS_World"))) "Undefined" 0 0))))

(event Custom|HurtTarget
  (params (OtherActor :type Actor%20Object%20Reference))
  (if (Actor|ActorHasTag OtherActor "PlayerProjectile")
    (Class|HealthComponent|TakeDamage (Variables|Default|GetHealthComponent) 25.0 false)
    (CallFunction|HealthBar)
    (bind _output_get (Variables|Default|SetTargetHitCount (+ (Variables|Default|GetTargetHitCount) 1)))
    (Development|PrintText (Utilities|Text|ToText(Integer) _output_get))
    (if (== (Variables|Default|GetTargetHitCount) 3)
      (Animation|PlayAnimMontage "/Game/Enemies/golemGetUp_Montage.golemGetUp_Montage" 1.0 "None"))))

(event Custom|WalkRight
  (Game|SpawnActorfromClass "/Game/Enemies/BP_MiniShockwave.BP_MiniShockwave_C" (Math|Transform|MakeTransform (.location (Transformation|GetSocketTransform (Variables|Character|GetMesh) "Foot_R" "RTS_World")) "0, 0, 0" "0.200000,0.200000,0.200000") "Undefined" 0 0))

(event Custom|WalkLeft
  (Game|SpawnActorfromClass "/Game/Enemies/BP_MiniShockwave.BP_MiniShockwave_C" (Math|Transform|MakeTransform (.location (Transformation|GetSocketTransform (Variables|Character|GetMesh) "Foot_L" "RTS_World")) "0, 0, 0" "0.200000,0.200000,0.200000") "Undefined" 0 0))

(event Custom|DestroyTarget
  (params (Target :type Static%20Mesh%20Component%20Object%20Reference))
  (Utilities|Array|RemoveItem (Variables|Default|GetTargets) Target)
  (Rendering|ToggleVisibility Target false)
  (Collision|SetCollisionEnabled Target "NoCollision")
  (Variables|Default|SetTargetHit? true))

(event Custom|HealthBar
  (CallFunction|UpdateHealthBar)
  (Utilities|FlowControl|Delay 1.0)
  (CallFunction|UpdateHealthBar2))

(event Custom|MoveToMiddle)

(event EventBeginPlay
  (bind _target2 (Variables|Default|GetTarget2))
  (Utilities|FlowControl|Sequence
    (:then_0
      (bind _asgolem_anim_bp (Utilities|Casting|CastToGolem_Anim_BP (Components|SkeletalMesh|GetAnimInstance (Variables|Character|GetMesh))))
      (Variables|/Game/Enemies/Golem_Anim_BP.Golem_Anim_BP_C|SetBossOBJ _asgolem_anim_bp self)
      (Collision|SetCollisionEnabled _target2 "NoCollision")
      (Rendering|ToggleVisibility _target2 false)
      (bind _returnvalue (UserInterface|CreateWidget "/Game/UI/Widget_BossHealth.Widget_BossHealth_C"))
      (Variables|/Game/UI/Widget_BossHealth.Widget_BossHealth_C|SetBoss%20Max%20Health _returnvalue (Variables|/Script/GP4.HealthComponent|GetMaxHealth (Variables|Default|GetHealthComponent)))
      (bind _output_get (Variables|Default|SetBossBarWidget _returnvalue))
      (UserInterface|Viewport|AddtoViewport _output_get 0)
      (CallFunction|UpdateHealthBar)
      (CallFunction|UpdateHealthBar2))
    (:then_1
      (bind _blackboardcomponent (Class|AIController|UseBlackboard (AI|GetAIController (Pawn|GetController)) "/Game/Enemies/BehaviorTrees/BB_Boss.BB_Boss"))
      (AI|Components|Blackboard|SetValueasVector _blackboardcomponent (Utilities|Name|MakeLiteralName "ArenaMiddle") (Transformation|GetWorldLocation (Variables|/Game/Enemies/BP_BossReturnLocation.BP_BossReturnLocation_C|GetLoc (Variables|Default|GetMiddleLocation)))))))

(event EventTick
  (params (DeltaSeconds :type Float%20%28single-precision%29))
  (bind _returnvalue (Pawn|GetController))
  (bind _returnvalue_2 (AI|GetAIController _returnvalue))
  (Utilities|FlowControl|Sequence
    (:then_0
      (bind _asgolem_anim_bp (Utilities|Casting|CastToGolem_Anim_BP (Components|SkeletalMesh|GetAnimInstance (Variables|Character|GetMesh))))
      (Variables|/Game/Enemies/Golem_Anim_BP.Golem_Anim_BP_C|SetEnableWalkAnim _asgolem_anim_bp (Variables|Default|GetEnableWalk))
      (bind _blackboardcomponent (Class|AIController|UseBlackboard _returnvalue_2 "/Game/Enemies/BehaviorTrees/BB_Boss.BB_Boss"))
      (AI|Components|Blackboard|SetValueasBool _blackboardcomponent (Utilities|Name|MakeLiteralName "CanWalk?") (Variables|/Game/Enemies/Golem_Anim_BP.Golem_Anim_BP_C|GetCan%20walk _asgolem_anim_bp))
      (CallFunction|SetLaserEyeBeamEndLocation))
    (:then_1
      (CallFunction|SetStompAnimation))
    (:then_2
      (bind _blackboardcomponent_2 (Class|AIController|UseBlackboard _returnvalue_2 "/Game/Enemies/BehaviorTrees/BB_Boss.BB_Boss"))
      (AI|Components|Blackboard|SetValueasBool _blackboardcomponent_2 (Utilities|Name|MakeLiteralName "IsTargetHit?") (Variables|Default|GetTargetHit?))
      (if (Variables|Default|GetTargetHit?)
        (Utilities|FlowControl|Delay (Variables|Default|GetSunBeamPhaseLength))
        (Variables|Default|SetTargetHit? false)))
    (:then_3
      (bind _blackboardcomponent_3 (Class|AIController|UseBlackboard _returnvalue_2 "/Game/Enemies/BehaviorTrees/BB_Boss.BB_Boss"))
      (AI|Components|Blackboard|SetValueasBool _blackboardcomponent_3 (Utilities|Name|MakeLiteralName "Staggered?") (Variables|Default|GetStaggered?)))
    (:then_4
      (if (>= (Variables|Default|GetTargetHitCount) 3)
        (Variables|Default|SetStaggered? false)
        (Variables|Default|SetTargetHitCount 0)
        (CallFunction|DestroyTarget (Variables|Default|GetTarget2))
        (CallFunction|DestroyTarget (Variables|Default|GetRuneMat))))
    (:then_5
      (if (<= (Variables|/Script/GP4.HealthComponent|GetCurrentHealth (Variables|Default|GetHealthComponent)) 0.0)
        (CallFunction|MovetoMiddle)))))

(fn ConstructionScript)

(fn RemoveTargets)

(fn UpdateHealthBar
  (bind _aswidget_boss_health (Utilities|Casting|CastToWidget_BossHealth (Variables|Default|GetBossBarWidget)))
  (Variables|/Game/UI/Widget_BossHealth.Widget_BossHealth_C|SetHealth _aswidget_boss_health (Math|Float|Truncate (Variables|/Script/GP4.HealthComponent|GetCurrentHealth (Variables|Default|GetHealthComponent))))
  (return))

(fn UpdateHealthBar2
  (bind _aswidget_boss_health (Utilities|Casting|CastToWidget_BossHealth (Variables|Default|GetBossBarWidget)))
  (Variables|/Game/UI/Widget_BossHealth.Widget_BossHealth_C|SetHealth2 _aswidget_boss_health (Math|Float|Truncate (Variables|/Script/GP4.HealthComponent|GetCurrentHealth (Variables|Default|GetHealthComponent))))
  (return))