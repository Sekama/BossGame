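; Player character Blueprint, named as a main menu model, with crossbow combat, dashing, health and pause handling.
; Health, Fire and Dash component events drive montages, sounds, widget updates and a level reload on death.
; Right mouse toggles aiming, keys 5/6 change health, and Tick copies one projectile spawn's position to another.
; BeginPlay and InitWidget are empty; main widget creation is unreachable, though other graphs still reference that widget.
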(event OnHit(HealthComponent)
  (params (Damage :type Float%20%28single-precision%29) (bIsCrit :type Boolean))
  ;[1 1 1] Widgets
  (if (<= (Variables|/Script/GP4.HealthComponent|GetCurrentHealth (Variables|Default|GetHealthComponent)) 0.0)
    (bind _returnvalue (Game|GetCurrentLevelName true))
    (Game|OpenLevel(byName) (Utilities|String|StringToName _returnvalue))
    (else
      (Default|TakeDamage (Variables|/Game/UI/Widget_MainWidget.Widget_MainWidget_C|GetWidget_PlayerHealthWidget (Variables|Default|GetMainWidget))))))

(event OnGainHealth(HealthComponent)
  ;[1 1 1] Widgets
  (Default|GainHealth (Variables|/Game/UI/Widget_MainWidget.Widget_MainWidget_C|GetWidget_PlayerHealthWidget (Variables|Default|GetMainWidget))))

(event OnFire(FireComponent)
  (Animation|Montage|PlayMontage (Variables|Character|GetMesh) "/Game/Animation/Crossbow_attack3_Montage.Crossbow_attack3_Montage"
    (:then
      (Audio|PlaySound2D "/Game/Sounds/MetaSounds/PlayerWeaponFire_MSS.PlayerWeaponFire_MSS" 1.0 1.0 0.0 0 0))))

(event OnReloadStart(FireComponent)
  (Animation|Montage|PlayMontage (Variables|Character|GetMesh) "/Game/Animation/Crossbow_reload_Montage.Crossbow_reload_Montage" 2.0
    (:then
      (Audio|PlaySound2D "/Game/Sounds/MetaSounds/PlayerRandomWeaponReload_MSS.PlayerRandomWeaponReload_MSS" 1.0 1.0 0.0 0 0))))

(event OnDash(DashComponent)
  (params (bIsDashing :type Boolean))
  (if bIsDashing
    (Audio|PlaySound2D "/Game/Sounds/MetaSounds/PlayerDash_MSS.PlayerDash_MSS" 1.0 1.0 0.0 0 0)
    (Animation|Montage|PlayMontage (Variables|Character|GetMesh) "/Game/Animation/Crossbow_rollforward_Montage.Crossbow_rollforward_Montage"
      (:then
        (Default|ShowCrosshair (Variables|Default|GetMainWidget) false)
        (Variables|Default|SetIsAiming false)))))

(event Custom|Init%20Widget
  ;[1 1 1] Widgets
)

(event Custom|ShakeYabooty
  (Class|PlayerCharacter|ShakeCamera 0.1 5e+02))

(event EventBeginPlay
  ;[1 0.8637 0.4549] Initial Setup
)

(event EventOnPause
  (params (Pause :type Boolean))
  ;[1 1 1] Widgets
  (Variables|/Script/Engine.PlayerController|SetbShowMouseCursor (Game|GetPlayerController 0) Pause)
  (Game|SetGamePaused Pause)
  (if Pause
    (bind _returnvalue (UserInterface|CreateWidget "/Game/UI/Widget_PauseMenu.Widget_PauseMenu_C" (Game|GetPlayerController 0)))
    (bind _output_get (Variables|Default|SetMenuWidget _returnvalue))
    (UserInterface|Viewport|AddtoViewport _returnvalue 0)
    (else
      (Widget|RemovefromParent (Variables|Default|GetMenuWidget)))))

(event EventTick
  (params (DeltaSeconds :type Float%20%28single-precision%29))
  (Transformation|SetRelativeLocation (Variables|Default|GetProjectileSpawn) (Variables|/Script/Engine.SceneComponent|GetRelativeLocation (Variables|Default|GetProjectileSpawn1)) false true))

(event Input|MouseEvents|RightMouseButton
  (params (Key :type Key%20Structure :default "None"))
  (bind _dashcomponent (Variables|Default|GetDashComponent))
  (bind _mainwidget (Variables|Default|GetMainWidget))
  (bind _bisdashing (Variables|/Script/GP4.DashComponent|GetbIsDashing _dashcomponent))
  (:Pressed
    (if (not _bisdashing)
      (Default|ShowCrosshair _mainwidget true)
      (Variables|Default|SetIsAiming true)))
  (:Released
    (if (not _bisdashing)
      (Default|ShowCrosshair _mainwidget false)
      (Variables|Default|SetIsAiming false))))

(event Input|KeyboardEvents|5
  (params (Key :type Key%20Structure :default "None"))
  (:Pressed
    (Class|HealthComponent|TakeDamage (Variables|Default|GetHealthComponent) 1.0 false)))

(event Input|KeyboardEvents|6
  (params (Key :type Key%20Structure :default "None"))
  (:Pressed
    (Class|HealthComponent|GainHealth (Variables|Default|GetHealthComponent) 1)))

(fn ConstructionScript)