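; Player character Blueprint for a crossbow-wielding hero, tying health, firing and dash components to animation and UI.
; Creates the main HUD on start, forwards damage and healing to its health widget, and reloads the current level on death.
; Fire, reload and dash events play crossbow montages, while right mouse toggles aiming and the crosshair.
; Also handles pausing with a menu widget and includes debug keys for damage and healing.
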(event OnHit(HealthComponent)
  (params (Damage :type Float%20%28single-precision%29) (bIsCrit :type Boolean))
  ;[1 1 1] Widgets
  (if (<= (Variables|/Script/GP4.HealthComponent|GetCurrentHealth (Variables|Default|GetHealthComponent)) 0.0)
    (bind _returnvalue (Game|GetCurrentLevelName true))
    (Game|OpenLevel(byName) (Utilities|String|StringToName _returnvalue))
    (else
      (Default|TakeDamage (Variables|/Game/UI/Widget_MainWidget.Widget_MainWidget_C|GetWidget_PlayerHealthWidget (Variables|Default|GetMainWidget))))))

(event OnGainHealth(HealthComponent)
  ;[1 1 1] Widgets
  (Default|GainHealth (Variables|/Game/UI/Widget_MainWidget.Widget_MainWidget_C|GetWidget_PlayerHealthWidget (Variables|Default|GetMainWidget))))

(event OnFire(FireComponent)
  (Animation|Montage|PlayMontage (Variables|Character|GetMesh) "/Game/Animation/Crossbow_attack3_Montage.Crossbow_attack3_Montage"))

(event OnReloadStart(FireComponent)
  (Animation|Montage|PlayMontage (Variables|Character|GetMesh) "/Game/Animation/Crossbow_reload_Montage.Crossbow_reload_Montage" 2.0))

(event OnDash(DashComponent)
  (params (bIsDashing :type Boolean))
  (if bIsDashing
    (Animation|Montage|PlayMontage (Variables|Character|GetMesh) "/Game/Animation/Crossbow_rollforward_Montage.Crossbow_rollforward_Montage"
      (:then
        (Development|PrintString "Hello")))))

(event Custom|Init%20Widget
  (bind _returnvalue (Game|GetPlayerController 0))
  ;[1 1 1] Widgets
  (bind _returnvalue_2 (UserInterface|CreateWidget "/Game/UI/Widget_MainWidget.Widget_MainWidget_C" _returnvalue (Math|Float|Round (Variables|/Script/GP4.HealthComponent|GetMaxHealth (Variables|Default|GetHealthComponent))) self))
  (bind _output_get (Variables|Default|SetMainWidget _returnvalue_2))
  (UserInterface|Viewport|AddtoViewport _output_get 0)
  (bind _returnvalue_3 (UserInterface|CreateWidget "/Game/UI/Widget_PauseMenu.Widget_PauseMenu_C" _returnvalue))
  (Variables|Default|SetMenuWidget _returnvalue_3))

(event Custom|ShakeYabooty
  (Class|PlayerCharacter|ShakeCamera 0.1 1e+02))

(event EventBeginPlay
  (CallFunction|InitWidget))

(event EventOnPause
  (params (Pause :type Boolean))
  ;[1 1 1] Widgets
  (Variables|/Script/Engine.PlayerController|SetbShowMouseCursor (Game|GetPlayerController 0) Pause)
  (Game|SetGamePaused Pause)
  (if Pause
    (bind _returnvalue (UserInterface|CreateWidget "/Game/UI/Widget_PauseMenu.Widget_PauseMenu_C" (Game|GetPlayerController 0)))
    (bind _output_get (Variables|Default|SetMenuWidget _returnvalue))
    (UserInterface|Viewport|AddtoViewport _returnvalue 0)
    (else
      (Widget|RemovefromParent (Variables|Default|GetMenuWidget)))))

(event EventTick
  (params (DeltaSeconds :type Float%20%28single-precision%29))
  (Transformation|SetRelativeLocation (Variables|Default|GetProjectileSpawn) (Variables|/Script/Engine.SceneComponent|GetRelativeLocation (Variables|Default|GetProjectileSpawn1)) false false))

(event Input|MouseEvents|RightMouseButton
  (params (Key :type Key%20Structure :default "None"))
  (bind _mainwidget (Variables|Default|GetMainWidget))
  (:Pressed
    (Default|ShowCrosshair _mainwidget true)
    (Variables|Default|SetIsAiming true))
  (:Released
    (Default|ShowCrosshair _mainwidget false)
    (Variables|Default|SetIsAiming false)))

(event Input|KeyboardEvents|5
  (params (Key :type Key%20Structure :default "None"))
  (:Pressed
    (Class|HealthComponent|TakeDamage (Variables|Default|GetHealthComponent) 1.0 false)))

(event Input|KeyboardEvents|6
  (params (Key :type Key%20Structure :default "None"))
  (:Pressed
    (Class|HealthComponent|GainHealth (Variables|Default|GetHealthComponent) 1)))

(fn ConstructionScript)