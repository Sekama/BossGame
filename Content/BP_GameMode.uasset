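; Game mode that runs the theme music and the transition into the boss's second phase, triggered automatically shortly after BeginPlay.
; SetMusic mixes five track volumes and a master volume through parameters on the spawned sound.
; InitializePhase2 triggers SandFloor, switches to a transition camera, teleports and freezes the player, and swaps the first boss for the hidden phase-two boss.
; SandFloor's completion event restores view, gravity and movement, then starts phase two.
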(event Custom|InitializePhase2
  (bind _returnvalue (Game|GetPlayerController 0))
  (bind _as_bp_player (Variables|Default|GetAs%20BP%20Player))
  (Default|BlackoutFadeOut (Variables|/Game/Player/BP_Player.BP_Player_C|GetMainWidget (Variables|Default|GetAs%20BP%20Player)))
  (Class|Triggerable|Trigger (Variables|Default|GetSandFloor))
  (EventDispatchers|BindEventtoTriggerDone (Variables|Default|GetSandFloor) (delegate Custom|OnTriggerDone))
  (Variables|Default|SetOriginalView (Pawn|GetViewTarget _returnvalue))
  (Game|Player|SetViewTargetwithBlend _returnvalue (Variables|Default|GetTransitionCamera) 0.0 "VTBlend_Linear" 0.0 false)
  (Default|BlackoutFadein (Variables|/Game/Player/BP_Player.BP_Player_C|GetMainWidget (Variables|Default|GetAs%20BP%20Player)))
  (Transformation|Teleport _as_bp_player (Variables|Default|GetPhase2PlayerStartLocation) "0, 0, 0")
  (Variables|/Script/GP4.PlayerMovementComponent|SetbApplyGravity (Variables|/Script/GP4.PlayerCharacter|GetMovementComponent _as_bp_player) false)
  (Rendering|SetActorHiddenInGame (Variables|Default|GetPhaseTwo) false)
  (bind _returnvalue_2 (Actor|GetActorOfClass "/Game/Enemies/BP_Boss_First_NEW.BP_Boss_First_NEW_C"))
  (Actor|DestroyActor _returnvalue_2)
  (Variables|/Script/GP4.PlayerCharacter|SetbIsAllowedToMove (Variables|Default|GetAs%20BP%20Player) false))

(event Custom|OnTriggerDone
  (Game|Player|SetViewTargetwithBlend (Game|GetPlayerController 0) (Variables|Default|GetOriginalView) 0.5 "VTBlend_Linear" 0.0 false)
  (Variables|/Script/GP4.PlayerMovementComponent|SetbApplyGravity (Variables|/Script/GP4.PlayerCharacter|GetMovementComponent (Variables|Default|GetAs%20BP%20Player)) true)
  (Variables|/Script/Engine.CharacterMovementComponent|SetGravityScale (Variables|/Script/Engine.Character|GetCharacterMovement (Variables|Default|GetPhaseTwo)) 1.0)
  (Default|StartPhaseTwo (Variables|Default|GetPhaseTwo))
  (Variables|/Script/GP4.PlayerCharacter|SetbIsAllowedToMove (Variables|Default|GetAs%20BP%20Player) true))

(event Custom|TeleportPlayerToPhase2)

(event EventBeginPlay
  (bind _asbp_player (Utilities|Casting|CastToBP_Player (Game|Player|GetPlayerPawn 0)))
  (Variables|Default|SetAs%20BP%20Player _asbp_player)
  (bind _returnvalue (Audio|SpawnSound2D "/Game/Sounds/MetaSounds/ThemeMusicV2_MSS.ThemeMusicV2_MSS" 1.0 1.0 0.0 0))
  (Variables|Default|SetBGM _returnvalue)
  (CallFunction|SetMusic (Variables|Arrangements|GetArrangement) 0.2)
  (bind _returnvalue_2 (Actor|GetActorOfClass "/Game/Enemies/BP_Boss_First_PhaseTwo.BP_Boss_First_PhaseTwo_C"))
  (bind _output_get (Variables|Default|SetPhaseTwo _returnvalue_2))
  (Rendering|SetActorHiddenInGame _output_get true)
  (Variables|/Script/Engine.CharacterMovementComponent|SetGravityScale (Variables|/Script/Engine.Character|GetCharacterMovement _output_get) 0.0)
  (Utilities|FlowControl|Delay 2.0)
  (CallFunction|InitializePhase2))

(fn ConstructionScript)

(fn SetMusic
  (params (New%20Arrangement :type Music%20Arrangement%20Structure) (Master%20Volume :type Float%20%28double-precision%29))
  (bind _bgm (Variables|Default|GetBGM))
  (Audio|Parameter|SetFloatParameter _bgm "VolumeTrack01" (.volume1 New%20Arrangement) :!class /Script/AudioExtensions.AudioParameterControllerInterface)
  (Audio|Parameter|SetFloatParameter _bgm "VolumeTrack02" (.volume2 New%20Arrangement) :!class /Script/AudioExtensions.AudioParameterControllerInterface)
  (Audio|Parameter|SetFloatParameter _bgm "VolumeTrack03" (.volume3 New%20Arrangement) :!class /Script/AudioExtensions.AudioParameterControllerInterface)
  (Audio|Parameter|SetFloatParameter _bgm "VolumeTrack04" (.volume4 New%20Arrangement) :!class /Script/AudioExtensions.AudioParameterControllerInterface)
  (Audio|Parameter|SetFloatParameter _bgm "VolumeTrack05" (.volume5 New%20Arrangement) :!class /Script/AudioExtensions.AudioParameterControllerInterface)
  (Audio|Parameter|SetFloatParameter _bgm "MasterVolume" Master%20Volume :!class /Script/AudioExtensions.AudioParameterControllerInterface))